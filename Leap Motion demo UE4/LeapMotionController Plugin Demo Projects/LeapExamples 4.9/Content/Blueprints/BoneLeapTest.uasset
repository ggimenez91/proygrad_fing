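; BoneLeapTest is a debug actor for Leap bone tracking that reports the index fingertip position.
; Tick accumulates delta time and, about once per second, prints the actor's world location if its LeapBoneType is Finger1Tip.
; Overlap, BeginPlay and construction logic are empty.
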(event `self.ReceiveActorBeginOverlap`
  (params (OtherActor :type "Actor Object Reference")))

(event `self.ReceiveBeginPlay`)

(event `self.ReceiveTick`
  (params (DeltaSeconds :type "Float (single-precision)"))
  (bind _output_get (set `self.t` (+ DeltaSeconds (`self.t`))))
  (if (and (>= _output_get 1.0) (`|EnumEquality` (`self.LeapBoneType`) "Finger1Tip"))
    (set `self.t` 0.0)
    (`KismetSystemLibrary.PrintString` (`KismetStringLibrary.Concat_StrStr` "Indice pos: " (`KismetStringLibrary.Conv_VectorToString` (`self.K2_GetActorLocation`))))))

(fn `UserConstructionScript`)